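; TargetDummy is a damageable target actor that can be destroyed.
; Its AnyDamage event subtracts incoming damage from Health and plays a damage sound at the actor's location.
; When Health drops to zero or below, it calls OnDeath, which plays an explosion sound and destroys the actor.
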(event Custom|OnDeath
  (Audio|PlaySoundatLocation (Variables|Default|GetExplosionSound) (Transformation|GetActorLocation))
  (Actor|DestroyActor))

(event Game|Damage|EventAnyDamage
  (params (Damage :type Float%20%28single-precision%29) (DamageType :type Damage%20Type%20Object%20Reference) (InstigatedBy :type Controller%20Object%20Reference) (DamageCauser :type Actor%20Object%20Reference))
  (Variables|Default|SetHealth (- (Variables|Default|GetHealth) Damage))
  (Audio|PlaySoundatLocation (Variables|Default|GetDamageSound) (Transformation|GetActorLocation))
  (if (<= (Variables|Default|GetHealth) 0.0)
    (CallFunction|OnDeath)))

(fn ConstructionScript)