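; DadSonHUD is a HUD Blueprint that gives each player a pilot or gunner interface.
; On BeginPlay it reads IsPilot from the owning DadSonPlayerControllerBP, then creates either the ship or gunner widget and adds it to that player's screen.
; Tick compares ShowHUD with a cached copy and shows or hides the widget only when the value changes.
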(event EventBeginPlay
  (Utilities|FlowControl|Sequence
    (:then_0
      (bind _asdad_son_player_controller_bp (Utilities|Casting|CastToDadSonPlayerControllerBP (Game|Player|GetOwningPlayerController)))
      (bind _returnvalue (UserInterface|CreateWidget (select (Variables|/Game/DadSonBP/Blueprints/DadSonPlayerControllerBP.DadSonPlayerControllerBP_C|GetbIsPilot _asdad_son_player_controller_bp) (Variables|Default|GetShipWidgetClass) (Variables|Default|GetGunnerWidgetClass)) (Game|Player|GetOwningPlayerController)))
      (UserInterface|Viewport|AddtoPlayerScreen _returnvalue)
      (Variables|Default|SetCurrentWidget _returnvalue)
      (Variables|Default|SetCachedShowHUD (Variables|Default|GetbShowHUD)))))

(event EventTick
  (params (DeltaSeconds :type Float%20%28single-precision%29))
  (bind _currentwidget (Variables|Default|GetCurrentWidget))
  (bind _bshowhud (Variables|Default|GetbShowHUD))
  (if (not (Math|Boolean|Equal(Boolean) _bshowhud (Variables|Default|GetCachedShowHUD)))
    (bind _output_get (Variables|Default|SetCachedShowHUD _bshowhud))
    (if _output_get
      (Widget|SetVisibility _currentwidget "Visible")
      (else
        (Widget|SetVisibility _currentwidget "Hidden")))))

(fn ConstructionScript)