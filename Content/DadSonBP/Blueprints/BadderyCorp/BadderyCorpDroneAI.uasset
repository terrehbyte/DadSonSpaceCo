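; AI controller for the Baddery Corp drone that detects a flying pawn and chases it.
; A detection sphere, sized by DetectionRadius at construction, locks onto the first FlyingPawn to overlap it while no valid target exists.
; Each tick, it steers the drone straight at the target through FloatingPawnMovement until within AcceptanceRadius, without pathfinding.
; Random player targeting is present but unconnected.
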(event OnComponentBeginOverlap(DetectionVolume)
  (params (OverlappedComponent :type Primitive%20Component%20Object%20Reference) (OtherActor :type Actor%20Object%20Reference) (OtherComp :type Primitive%20Component%20Object%20Reference) (OtherBodyIndex :type Integer) (bFromSweep :type Boolean) (SweepResult :type Hit%20Result%20Structure%20%28by%20ref%29))
  (Utilities|IsValid (Variables|Default|GetTarget)
    (:Is%20Not%20Valid
      (bind _asflying_pawn (Utilities|Casting|CastToFlyingPawn OtherActor))
      (Variables|Default|SetTarget _asflying_pawn)
      (Development|PrintString "Target acquired."))))

(event EventBeginPlay)

(event EventTick
  (params (DeltaSeconds :type Float%20%28single-precision%29))
  (bind _returnvalue (Pawn|GetControlledPawn))
  (if (>= (Transformation|GetDistanceTo self (Variables|Default|GetTarget)) (Variables|AI|GetAcceptanceRadius))
    (Utilities|IsValid (Variables|Default|GetTarget)
      (:Is%20Valid
        (bind _asbaddery_drone_bp (Utilities|Casting|CastToBadderyDroneBP _returnvalue))
        (Class|PawnMovementComponent|AddInputVector (Variables|/Game/DadSonBP/Blueprints/BadderyCorp/BadderyDroneBP.BadderyDroneBP_C|GetFloatingPawnMovement _asbaddery_drone_bp) (Math|Vector|GetUnitDirection(Vector) (Transformation|GetActorLocation _returnvalue) (Transformation|GetActorLocation (Variables|Default|GetTarget))) false)))))

(fn ConstructionScript
  (Components|Sphere|SetSphereRadius (Variables|AI|GetDetectionVolume) (Variables|AI|GetDetectionRadius) true))