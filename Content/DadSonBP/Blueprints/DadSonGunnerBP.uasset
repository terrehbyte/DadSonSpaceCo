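; Gunner pawn that rides on the FlyingPawn flown by the Dad controller and shoots with a movable screen crosshair.
; On possession it snaps to that pawn's GunnerPosition and caches the gunner HUD's crosshair slot.
; Aim axes slide the crosshair by shifting its clamped canvas anchors, both using AimUpRate.
; Fire is interval-limited and line-traces from the HUD's crosshair ray, damaging hit Pawn or Destructible objects.
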(event EventPossessed
  (params (NewController :type Controller%20Object%20Reference))
  (bind _returnvalue (Pawn|GetController))
  (bind _asdad_son_player_controller_bp (Utilities|Casting|CastToDadSonPlayerControllerBP _returnvalue)
    (:then
      (bind _asflying_pawn (Utilities|Casting|CastToFlyingPawn (Pawn|GetControlledPawn (Variables|/Game/DadSonBP/Blueprints/DadSonPlayerControllerBP.DadSonPlayerControllerBP_C|GetDadController _asdad_son_player_controller_bp))))
      (Transformation|AttachComponentToComponent (Variables|/Game/FlyingBP/Blueprints/FlyingPawn.FlyingPawn_C|GetGunnerPosition _asflying_pawn) "None" "SnapToTarget" "SnapToTarget" "SnapToTarget" true)
      (bind _asdad_son_hud (Utilities|Casting|CastToDadSonHUD (HUD|GetHUD (.AsDad%20Son%20Player%20Controller%20BP (Utilities|Casting|CastToDadSonPlayerControllerBP (Pawn|GetController))))))
      (bind _asdad_son_gunner_hudbp (Utilities|Casting|CastToDadSonGunnerHUDBP (Variables|/Game/DadSonBP/Blueprints/DadSonHUD.DadSonHUD_C|GetCurrentWidget _asdad_son_hud)))
      (Variables|Reticule|SetReticuleSlot (Class|WidgetLayoutLibrary|SlotasCanvasSlot (Variables|/Game/DadSonBP/Widgets/DadSonGunnerHUDBP.DadSonGunnerHUDBP_C|GetCrosshair _asdad_son_gunner_hudbp)))
      (Variables|Reticule|SetHUD _asdad_son_gunner_hudbp))
    (:CastFailed
      (Development|PrintString (Utilities|String|BuildString(Object) "No dice, here's what you got instead: " (Utilities|GetDisplayName _returnvalue) 0)))))

(event EventBeginPlay
  (Development|PrintString "Gunner spawned."))

(event Input|ActionEvents|InputActionFire
  (params (Key :type Key%20Structure))
  (:Pressed
    (if (CallFunction|CanFire)
      (Variables|Firing|SetNextFireTime (+ (Utilities|Time|GetGameTimeinSeconds) (Variables|Firing|GetFireInterval)))
      (Audio|PlaySound2D self (Variables|Firing|GetFireCue) 1e+01 1.0 0.0 0 self)
      (bind (_position _direction) (Default|GetTraceDataUnderCrosshair (Variables|Reticule|GetHUD)))
      (bind (_outhit _returnvalue) (Collision|LineTraceForObjects _position (+ _position (* _direction (Variables|Firing|GetMaxFireDistance))) (Utilities|Array|MakeArray "ObjectTypeQuery3" "ObjectTypeQuery6") true 0 "ForOneFrame"))
      (if _returnvalue
        (Game|Damage|ApplyDamage (.HitActor (Collision|BreakHitResult _outhit)) (Variables|Firing|GetDamagePerShot) (Pawn|GetController) self "/Script/Engine.DamageType")))))

(event Input|AxisEvents|InputAxisAimUp
  (params (AxisValue :type Float%20%28single-precision%29))
  (bind _returnvalue (Utilities|Time|GetWorldDeltaSeconds))
  (bind _reticuleslot (Variables|Reticule|GetReticuleSlot))
  (bind _aimuprate (Variables|Reticule|GetAimUpRate))
  (bind _returnvalue_2 (Class|CanvasPanelSlot|GetAnchors _reticuleslot))
  (bind _returnvalue_3 (* AxisValue _aimuprate _returnvalue))
  (bind _maximum (Utilities|Struct|BreakAnchors _returnvalue_2))
  (bind _returnvalue_4 (Math|Vector2D|MakeVector2D 0.0 _returnvalue_3))
  (bind _returnvalue_5 (+ _returnvalue_4 _maximum))
  (bind (_x _y) (Math|Vector2D|BreakVector2D _returnvalue_5))
  (bind _returnvalue_6 (Math|Float|Clamp(Float) _x))
  (bind _returnvalue_7 (Math|Float|Clamp(Float) _y))
  (bind _returnvalue_8 (Math|Vector2D|MakeVector2D _returnvalue_6 _returnvalue_7))
  (Utilities|IsValid (Variables|Reticule|GetReticuleSlot)
    (:Is%20Valid
      (Class|CanvasPanelSlot|SetAnchors (Variables|Reticule|GetReticuleSlot) (Utilities|Struct|MakeAnchors _returnvalue_8 _returnvalue_8)))))

(event Input|AxisEvents|InputAxisAimRight
  (params (AxisValue :type Float%20%28single-precision%29))
  (bind _returnvalue (Utilities|Time|GetWorldDeltaSeconds))
  (bind _aimuprate (Variables|Reticule|GetAimUpRate))
  (bind _reticuleslot (Variables|Reticule|GetReticuleSlot))
  (bind _returnvalue_2 (Class|CanvasPanelSlot|GetAnchors _reticuleslot))
  (bind _returnvalue_3 (* AxisValue _aimuprate _returnvalue))
  (bind _maximum (Utilities|Struct|BreakAnchors _returnvalue_2))
  (bind _returnvalue_4 (Math|Vector2D|MakeVector2D _returnvalue_3 0.0))
  (bind _returnvalue_5 (+ _returnvalue_4 _maximum))
  (bind (_x _y) (Math|Vector2D|BreakVector2D _returnvalue_5))
  (bind _returnvalue_6 (Math|Float|Clamp(Float) _y))
  (bind _returnvalue_7 (Math|Float|Clamp(Float) _x))
  (bind _returnvalue_8 (Math|Vector2D|MakeVector2D _returnvalue_7 _returnvalue_6))
  (Utilities|IsValid (Variables|Reticule|GetReticuleSlot)
    (:Is%20Valid
      (Class|CanvasPanelSlot|SetAnchors (Variables|Reticule|GetReticuleSlot) (Utilities|Struct|MakeAnchors _returnvalue_8 _returnvalue_8)))))

(fn ConstructionScript)

(fn CanFire
  (return (>= (Utilities|Time|GetGameTimeinSeconds) (Variables|Firing|GetNextFireTime))))