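; Game mode for a local two-player pilot-and-gunner game, spawning a second local player at BeginPlay.
; On login it alternates controllers between pilot and gunner by ship and gunner counts, linking each gunner to the last pilot's controller and decrementing counts on logout.
; Default pawn class follows that role, falling back to spectator.
; GameHasEnded disables pilot input, removes the gunner player and shows the game-over widget with mouse cursor.
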(event Custom|GameHasEnded
  (bind _returnvalue (Game|GetPlayerController 0))
  (bind _asflying_pawn (Utilities|Casting|CastToFlyingPawn (Game|Player|GetPlayerPawn 0)))
  (Input|DisableInput _asflying_pawn _returnvalue)
  (bind _outactors (Actor|GetAllActorsOfClass "/Game/DadSonBP/Blueprints/DadSonGunnerBP.DadSonGunnerBP_C"))
  (bind _asplayer_controller (Utilities|Casting|CastToPlayerController (Pawn|GetController (Utilities|Array|Get(acopy) _outactors))))
  (Class|GameplayStatics|RemovePlayer _asplayer_controller false)
  (bind _returnvalue_2 (UserInterface|CreateWidget "/Game/FlyingBP/Blueprints/W_GameOverBP.W_GameOverBP_C" _returnvalue))
  (bind _output_get (Variables|Default|SetGameOverWBP _returnvalue_2))
  (UserInterface|Viewport|AddtoPlayerScreen _output_get)
  (Variables|/Script/Engine.PlayerController|SetbShowMouseCursor (Game|GetPlayerController 0) true))

(event EventBeginPlay
  (Class|GameplayStatics|CreatePlayer -1))

(event EventTick
  (params (DeltaSeconds :type Float%20%28single-precision%29)))

(event EventOnLogout
  (params (ExitingController :type Controller%20Object%20Reference))
  (bind _asdad_son_player_controller_bp (Utilities|Casting|CastToDadSonPlayerControllerBP ExitingController))
  (if (Variables|/Game/DadSonBP/Blueprints/DadSonPlayerControllerBP.DadSonPlayerControllerBP_C|GetbIsPilot _asdad_son_player_controller_bp)
    (Variables|Default|SetShipCount (- (Variables|Default|GetShipCount) 1))
    (else
      (Variables|Default|SetGunnerCount (- (Variables|Default|GetGunnerCount) 1)))))

(event EventPostLogin
  (params (NewPlayer :type Player%20Controller%20Object%20Reference))
  (bind _asdad_son_player_controller_bp (Utilities|Casting|CastToDadSonPlayerControllerBP NewPlayer)
    (:then
      (bind _output_get (Variables|/Game/DadSonBP/Blueprints/DadSonPlayerControllerBP.DadSonPlayerControllerBP_C|SetbIsPilot _asdad_son_player_controller_bp (<= (Variables|Default|GetShipCount) (Variables|Default|GetGunnerCount))))
      (if _output_get
        (Variables|Default|SetLastShipController _asdad_son_player_controller_bp)
        (Math|Integer|IncrementInt (Variables|Default|GetShipCount))
        (else
          (Variables|/Game/DadSonBP/Blueprints/DadSonPlayerControllerBP.DadSonPlayerControllerBP_C|SetDadController _asdad_son_player_controller_bp (Variables|Default|GetLastShipController))
          (Math|Integer|IncrementInt (Variables|Default|GetGunnerCount)))))
    (:CastFailed
      (Development|PrintString "Player controller is not Dad or Son, no changes will be made."))))

(fn ConstructionScript)

(fn GetDefaultPawnClassforController
  (params (InController :type Controller%20Object%20Reference))
  (bind _asdad_son_player_controller_bp (Utilities|Casting|CastToDadSonPlayerControllerBP InController)
    (:then
      (return (select (Variables|/Game/DadSonBP/Blueprints/DadSonPlayerControllerBP.DadSonPlayerControllerBP_C|GetbIsPilot _asdad_son_player_controller_bp) (Variables|Default|GetShipClass) (Variables|Default|GetGunnerClass))))
    (:CastFailed
      (return "/Script/Engine.SpectatorPawn"))))